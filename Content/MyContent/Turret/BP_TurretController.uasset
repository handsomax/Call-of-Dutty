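; AI controller for the turret that runs its behavior tree on possess and feeds it perception and death state through the Blackboard.
; Sensing a FirstPersonCharacter records the enemy and its location and cancels the lose-sight timer.
; Any other perception update restarts that timer, which clears the enemy on expiry, so brief line-of-sight breaks are tolerated.
; The turret health component's death event sets the dead key.
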(event OnTargetPerceptionUpdated(AIPerception)
  (params (Actor :type Actor%20Object%20Reference) (Stimulus :type AI%20Stimulus%20Structure))
  (bind (_age _expirationage _strength _stimuluslocation _receiverlocation _tag _bsuccessfullysensed) (Utilities|Struct|BreakAIStimulus Stimulus))
  ;[1 1 1] Checks if Turret sees the player
  (if (and (== (Utilities|GetClass Actor) "/Game/MyContent/Blueprint/FirstPersonCharacter.FirstPersonCharacter_C") _bsuccessfullysensed)
    ;[1 1 1] The AI sees the player. It is recorded in the blackboard
    (CallFunction|SetSeesEnemy true Actor _stimuluslocation)
    (Utilities|Time|ClearandInvalidateTimerbyHandle (Variables|Default|GetBreakLineOfSightTimer))
    (else
      ;[1 1 1] The AI does not see the player. Wait for a bit
      (bind _returnvalue (Utilities|Time|SetTimerbyEvent (delegate Custom|BreakLineOfSight) (Variables|Default|GetTimeToLoseLineOfSight)))
      (Variables|Default|SetBreakLineOfSightTimer _returnvalue))))

(event Custom|BreakLineOfSight
  ;[1 1 1] Record in the blackboard that the AI does not see the player anymore
  (CallFunction|SetSeesEnemy false 0 "0, 0, 0"))

(event Custom|OnDeath
  (AI|Components|Blackboard|SetValueasBool (Variables|Default|GetBlackboard) (Variables|Default|GetDeadKey) true))

(event EventBeginPlay)

(event EventTick
  (params (DeltaSeconds :type Float%20%28single-precision%29)))

(event EventPossess
  (params (PossessedPawn :type Pawn%20Object%20Reference))
  (bind _asbp_turret (Utilities|Casting|CastToBP_turret PossessedPawn))
  (Variables|Default|SetAs%20BP%20Turret _asbp_turret)
  (AI|RunBehaviorTree "/Game/MyContent/Turret/BT_Turret.BT_Turret")
  (EventDispatchers|BindEventtoDeath (Variables|/Game/MyContent/Turret/BP_turret.BP_turret_C|GetBP_Health (Variables|Default|GetAs%20BP%20Turret)) (delegate Custom|OnDeath)))

(fn ConstructionScript)

(fn SetSeesEnemy
  (params (SeesEnemy :type Boolean) (Enemy :type Actor%20Object%20Reference) (EnemyPosition :type Vector))
  (bind _blackboard (Variables|Default|GetBlackboard))
  (AI|Components|Blackboard|SetValueasBool _blackboard (Variables|Default|GetSeesEnemyKey) SeesEnemy)
  (AI|Components|Blackboard|SetValueasObject _blackboard (Variables|Default|GetEnemyKey) Enemy)
  (AI|Components|Blackboard|SetValueasVector _blackboard (LocalVariables|GetEnemyPositionKey) EnemyPosition))

(fn MoveTowardEnemy)
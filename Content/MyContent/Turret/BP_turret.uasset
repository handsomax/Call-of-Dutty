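; Turret actor that aims its barrels, fires projectiles, takes damage and can explode.
; Timelines drive the search sweep and disabled droop, while helper functions interpolate aim toward a position or back to rest, returning whether it is reached.
; Shoot alternates between two barrel sockets to spawn first-person template projectiles with sound.
; Damage is forwarded to BPHealth, and Boom plays a one-time explosion effect and sound.
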(event Custom|Shoot
  (Game|SpawnActorfromClass "/Game/MyContent/Blueprint/FirstPersonProjectile.FirstPersonProjectile_C" (Math|Transform|MakeTransform (+ (.location (Transformation|GetSocketTransform (Variables|Default|GetBarrels) (select (Variables|Default|GetbBarrelToggle) "Barrel2" "Barrel1") "RTS_World")) (* (Math|Vector|GetForwardVector (.rotation (Transformation|GetSocketTransform (Variables|Default|GetBarrels) (select (Variables|Default|GetbBarrelToggle) "Barrel2" "Barrel1") "RTS_World"))) 2.0)) (.rotation (Transformation|GetSocketTransform (Variables|Default|GetBarrels) (select (Variables|Default|GetbBarrelToggle) "Barrel2" "Barrel1") "RTS_World")) (.scale (Transformation|GetSocketTransform (Variables|Default|GetBarrels) (select (Variables|Default|GetbBarrelToggle) "Barrel2" "Barrel1") "RTS_World"))) "Undefined" 0 0)
  (Variables|Default|SetbBarrelToggle (not (Variables|Default|GetbBarrelToggle)))
  (Audio|PlaySoundatLocation "/Game/FirstPerson/Audio/FirstPersonTemplateWeaponFire02.FirstPersonTemplateWeaponFire02" (Transformation|GetWorldLocation (Variables|Default|GetBarrels)) "0, 0, 0" 0.07 1.0 0.0 0 0 0) ; Play firing sound
)

(event Custom|StartSearch
  (bind _rotation (Timeline|SearchTimeline PlayFromStart)
    (:Update
      (Transformation|SetRelativeRotation (Variables|Default|GetBarrels) (Math|Rotator|MakeRotator 0.0 0.0 _rotation) false false))))

(event Custom|EndSearch
  (bind _rotation (Timeline|SearchTimeline Stop)
    (:Update
      (Transformation|SetRelativeRotation (Variables|Default|GetBarrels) (Math|Rotator|MakeRotator 0.0 0.0 _rotation) false false))))

(event Custom|Disable
  (bind _lookdown (Timeline|DisableTimeline PlayFromStart)
    (:Update
      (Transformation|SetRelativeRotation (Variables|Default|GetBarrels) (Math|Rotator|MakeRotator 0.0 _lookdown 0.0) false false))))

(event EventBeginPlay)

(event Collision|EventActorBeginOverlap
  (params (OtherActor :type Actor%20Object%20Reference)))

(event Game|Damage|EventAnyDamage
  (params (Damage :type Float%20%28single-precision%29) (DamageType :type Damage%20Type%20Object%20Reference) (InstigatedBy :type Controller%20Object%20Reference) (DamageCauser :type Actor%20Object%20Reference))
  (Development|PrintText (Utilities|Text|FormatText "Turret took {damage} damages" Damage))
  (Default|TakeDamage (Variables|Default|GetBP_Health) (Math|Float|Truncate Damage)))

(fn ConstructionScript)

(fn RotatetoFacePosition
  (params (Position :type Vector) (DeltaTime :type Float%20%28single-precision%29) (Speed :type Float%20%28single-precision%29))
  (bind _barrels (Variables|Default|GetBarrels))
  (bind _barrels_2 (Variables|Default|GetBarrels))
  (bind _returnvalue (Transformation|GetWorldLocation _barrels))
  (bind _returnvalue_2 (Transformation|GetWorldRotation _barrels_2))
  (bind _returnvalue_3 (Math|Rotator|FindLookatRotation _returnvalue Position))
  (bind _returnvalue_4 (Math|Interpolation|RInterpTo _returnvalue_2 _returnvalue_3 DeltaTime Speed))
  (Transformation|SetWorldRotation (Variables|Default|GetBarrels) _returnvalue_4 false false)
  (return (Math|Rotator|Equal(Rotator) _returnvalue_4 _returnvalue_3 1.0)))

(fn ResetPosition
  (params (Speed :type Float%20%28single-precision%29) (DeltaTime :type Float%20%28single-precision%29))
  (bind _barrels (Variables|Default|GetBarrels))
  (bind _relativerotation (Variables|/Script/Engine.SceneComponent|GetRelativeRotation _barrels))
  (bind _returnvalue (Math|Interpolation|RInterpTo _relativerotation "0, 0, 0" Speed DeltaTime))
  (Transformation|SetRelativeRotation _barrels _returnvalue false false)
  (return (Math|Rotator|Equal(Rotator) _returnvalue "0, 0, 0" 1.0)))

(fn Boom
  (Development|PrintString "BOOOOOOOM")
  (Utilities|FlowControl|DoOnce false
    (:Completed
      (Effects|SpawnEmitteratLocation "/Game/StarterContent/Particles/P_Explosion.P_Explosion" (Transformation|GetWorldLocation (Variables|Default|GetDefaultSceneRoot)) "0, 0, 0" "3.000000,3.000000,3.000000")
      (Audio|SpawnSoundAttached "/Game/MyContent/Visuals/Explosion/mixkit-explosion-hit-1704.mixkit-explosion-hit-1704" (Variables|Default|GetBase) "None" "0, 0, 0" "0, 0, 0" "KeepRelativeOffset" false 1.0 1.0 0.0 0 0))))
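; BP_Dutty is the level's goal: a skeletal-mesh character who calls for help until the player reaches it and wins.
; On BeginPlay it attaches a help-me sound to the mesh and keeps a reference to it.
; When the FirstPersonCharacter overlaps its Box, it freezes the player, swaps the help sound for dance music, loops a dance animation and shows the WB_WinMenu widget.
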(event OnComponentBeginOverlap(Box)
  (params (OverlappedComponent :type Primitive%20Component%20Object%20Reference) (OtherActor :type Actor%20Object%20Reference) (OtherComp :type Primitive%20Component%20Object%20Reference) (OtherBodyIndex :type Integer) (bFromSweep :type Boolean) (SweepResult :type Hit%20Result%20Structure%20%28by%20ref%29))
  (bind _skeletalmesh (Variables|Default|GetSkeletalMesh))
  (bind _asfirst_person_character (Utilities|Casting|CastToFirstPersonCharacter OtherActor))
  (Input|DisableInput _asfirst_person_character (Game|GetPlayerController 0))
  (Components|Movement|StopMovementImmediately (Variables|/Script/Engine.Character|GetCharacterMovement _asfirst_person_character))
  (Components|Animation|PlayAnimation (Variables|Default|GetSkeletalMesh) "/Game/MyContent/Blueprint/Dutty/Dancing_Maraschino_Step__1_.Dancing_Maraschino_Step__1_" true)
  (Audio|Components|Audio|Stop (Variables|Default|GetHelpSound))
  (Audio|SpawnSoundAttached "/Game/MyContent/Blueprint/Dutty/Danse_Madison__online-audio-converter_com_.Danse_Madison__online-audio-converter_com_" _skeletalmesh "None" (Transformation|GetWorldLocation _skeletalmesh) "0, 0, 0" "KeepRelativeOffset" false 0.2 1.0 0.0 0 0 false)
  (bind _returnvalue (UserInterface|CreateWidget "/Game/MyContent/Blueprint/widgets/WB_WinMenu.WB_WinMenu_C" (Game|GetPlayerController 0)))
  (UserInterface|Viewport|AddtoViewport _returnvalue 0))

(event EventBeginPlay
  (bind _skeletalmesh (Variables|Default|GetSkeletalMesh))
  (bind _returnvalue (Audio|SpawnSoundAttached "/Game/MyContent/Blueprint/Dutty/256030__pyro13djt__help-me.256030__pyro13djt__help-me" _skeletalmesh "None" (Transformation|GetWorldLocation _skeletalmesh) "0, 0, 0" "KeepRelativeOffset" false 0.2 1.0 0.0 0 0 false))
  (Variables|Default|SetHelpSound _returnvalue))

(fn ConstructionScript)
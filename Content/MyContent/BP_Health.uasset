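; BP_Health tracks a health value and signals death when it reaches zero.
; Health starts at MaxHealth on BeginPlay, and the TakeDamage and RecoverHealth events both pass their adjusted totals to SetHealth.
; As wired, SetHealth only acts when Dead is already true, clamping the value between zero and MaxHealth, then calling CallDeath and setting Dead at zero.
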(event Custom|TakeDamage
  (params (Damage :type Integer))
  (CallFunction|SetHealth (- (Variables|Default|GetHealth) Damage)))

(event Custom|SetHealth
  (params (Health :type Integer))
  (if (Variables|Default|GetDead)
    (bind _output_get (Variables|Default|SetHealth (Math|Integer|Clamp(Integer) Health 0 (Variables|Default|GetMaxHealth))))
    (if (== _output_get 0)
      (Default|CallDeath)
      (Variables|Default|SetDead true))))

(event Custom|RecoverHealth
  (params (HealhRecovered :type Integer))
  (CallFunction|SetHealth (+ HealhRecovered (Variables|Default|GetHealth))))

(event EventBeginPlay
  (Variables|Default|SetHealth (Variables|Default|GetMaxHealth)))

(event EventTick
  (params (DeltaSeconds :type Float%20%28single-precision%29)))